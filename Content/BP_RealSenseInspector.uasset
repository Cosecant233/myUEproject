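; RealSense camera inspector actor that shows raw depth, colorized depth, color and infrared textures on demo meshes.
; SetupDemoObjects binds each texture through a dynamic material, with optional background segmentation from depth and color.
; When enabled, the point cloud mesh is rotated and textured with color, or assigned colorized depth when color is off.
; Tick feeds the segmentation range into its material; overlapping the point cloud prints a debug string.
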(event OnComponentBeginOverlap(PclMesh)
  (params (OverlappedComponent :type Primitive%20Component%20Object%20Reference) (OtherActor :type Actor%20Object%20Reference) (OtherComp :type Primitive%20Component%20Object%20Reference) (OtherBodyIndex :type Integer) (bFromSweep :type Boolean) (SweepResult :type Hit%20Result%20Structure%20%28by%20ref%29))
  (Development|PrintString "Hello"))

(event EventBeginPlay)

(event EventTick
  (params (DeltaSeconds :type Float%20%28single-precision%29))
  (bind _bgsegmat (Variables|Default|GetBGSegMat))
  (Utilities|IsValid _bgsegmat
    (:Is%20Valid
      (Rendering|Material|SetScalarParameterValue _bgsegmat "MinRange" (Variables|Segmentation|GetSegMin) :!class /Script/Engine.MaterialInstanceDynamic)
      (Rendering|Material|SetScalarParameterValue _bgsegmat "MaxRange" (Variables|Segmentation|GetSegMax) :!class /Script/Engine.MaterialInstanceDynamic))))

(event EventEndPlay
  (params (EndPlayReason :type EEndPlayReason%20Enum :default "Destroyed")))

(fn ConstructionScript)

(fn SetDynamicMaterial
  (params (Object :type Primitive%20Component%20Object%20Reference) (Material :type Material%20Interface%20Object%20Reference) (Texture :type Texture%202D%20Object%20Reference) (ParamName :type String))
  (Utilities|IsValid Texture
    (:Is%20Valid
      (bind _returnvalue (Rendering|Material|CreateDynamicMaterialInstance Material "None" "None" :!class /Script/Engine.KismetMaterialLibrary))
      (Rendering|Material|SetMaterial Object 0 _returnvalue)
      (Rendering|Material|SetTextureParameterValue _returnvalue (Utilities|String|StringToName ParamName) Texture))))

(fn SetupDemoObjects
  (Utilities|FlowControl|Sequence
    (:then_0
      ;[1 1 1] Setup materials
      (CallFunction|SetDynamicMaterial (Variables|Default|GetDepthRawMesh) "/Game/M_Depth.M_Depth" (Variables|Default|GetDepthRawTexture) "DepthRaw")
      (CallFunction|SetDynamicMaterial (Variables|Default|GetColorMesh) "/Game/M_Color.M_Color" (Variables|Default|GetColorTexture) "Color")
      (CallFunction|SetDynamicMaterial (Variables|Default|GetDepthColorizedMesh) "/Game/M_Color.M_Color" (Variables|Default|GetDepthColorizedTexture) "Color")
      (CallFunction|SetDynamicMaterial (Variables|Default|GetInfraredMesh) "/Game/M_Infrared.M_Infrared" (Variables|Default|GetInfraredTexture) "Infrared"))
    (:then_1
      ;[1 1 1] Background segmentation
      (if (and (Variables|Default|GetbEnableRawDepth) (Variables|Default|GetbEnableColor))
        (bind _returnvalue (Rendering|Material|CreateDynamicMaterialInstance "/Game/M_BGSeg.M_BGSeg" "None" "None" :!class /Script/Engine.KismetMaterialLibrary))
        (Variables|Default|SetBGSegMat _returnvalue)
        (Rendering|Material|SetMaterial (Variables|Default|GetBGSegMesh) 0 _returnvalue)
        (Rendering|Material|SetTextureParameterValue (Variables|Default|GetBGSegMat) "DepthRaw" (Variables|Default|GetDepthRawTexture))
        (Rendering|Material|SetTextureParameterValue (Variables|Default|GetBGSegMat) "Color" (Variables|Default|GetColorTexture))
        (Rendering|Material|SetScalarParameterValue (Variables|Default|GetBGSegMat) "DepthScale" (Variables|Default|GetDepthScale) :!class /Script/Engine.MaterialInstanceDynamic)))
    (:then_2
      ;[1 1 1] PointCloud
      (if (Variables|Default|GetbEnablePcl)
        (Transformation|SetRelativeRotation (Variables|Default|GetPclMesh) "0,180.000000, 0" false false)
        (if (Variables|Default|GetbEnableColor)
          (bind _returnvalue_2 (Rendering|Material|CreateDynamicMaterialInstance "/Game/M_Color.M_Color" "None" "None" :!class /Script/Engine.KismetMaterialLibrary))
          (Class|RealSenseInspector|SetPointCloudMaterial 0 _returnvalue_2)
          (Rendering|Material|SetTextureParameterValue _returnvalue_2 "Color" (Variables|Default|GetColorTexture))
          (Transformation|SetRelativeRotation (Variables|Default|GetPclMesh) "0.000000,-180.000000,-90.000000" false false)
          (else
            (bind _returnvalue_3 (Rendering|Material|CreateDynamicMaterialInstance "/Game/M_Depth.M_Depth" "None" "None" :!class /Script/Engine.KismetMaterialLibrary))
            (Class|RealSenseInspector|SetPointCloudMaterial 0 _returnvalue_3)
            (Rendering|Material|SetTextureParameterValue _returnvalue_3 "Color" (Variables|Default|GetDepthColorizedTexture))))))))