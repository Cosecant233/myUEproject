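; Example actor demonstrating the RealSense camera plugin API through a BP_RealSenseInspector found in the level.
; BeginPlay gets the RealSense context, locates the inspector, then starts it and sets up its demo objects.
; Example functions, bundled in ExampleCollection but not called at runtime, show device enumeration, option changes, preset save/load, stream configuration and timer-driven record-then-playback.
; Unwired EventGraph snippets serve as further API samples.
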(event EventBeginPlay
  (CallFunction|InitContext)
  (CallFunction|InitInspector)
  (CallFunction|RunRealSenseDemo))

(event EventTick
  (params (DeltaSeconds :type Float%20%28single-precision%29)))

(fn ConstructionScript)

(fn ExEnumerateHardware
  (bind _context (Variables|Default|GetContext))
  ;[1 1 1] Enumerate devices
  (Class|RealSenseContext|QueryDevices _context)
  (for _array_element (Variables|/Script/RealSense.RealSenseContext|GetDevices _context)
    (Development|PrintString (Utilities|String|Append "DEVICE " (Variables|/Script/RealSense.RealSenseDevice|GetName _array_element) " SN: " (Variables|/Script/RealSense.RealSenseDevice|GetSerial _array_element)) false)
    ;[1 1 1] Enumerate sensors
    (for _array_element_2 (Variables|/Script/RealSense.RealSenseDevice|GetSensors _array_element)
      (Development|PrintString (Utilities|String|Append "SENSOR " (Variables|/Script/RealSense.RealSenseSensor|GetName _array_element_2)) false))))

(fn InitContext
  (Utilities|IsValid (Variables|Default|GetContext)
    (:Is%20Valid
      _)
    (:Is%20Not%20Valid
      (bind _returnvalue (Class|RealSenseContext|GetRealSense))
      (Variables|Default|SetContext _returnvalue)))
  (return (Variables|Default|GetContext)))

(fn ExampleCollection
  (Utilities|FlowControl|Sequence
    (:then_0
      (CallFunction|ExEnumerateHardware))
    (:then_1
      (CallFunction|ExModifyOption))
    (:then_2
      (CallFunction|ExPresetLoadSave))
    (:then_3
      (CallFunction|ExStreamConfiguration))
    (:then_4
      (CallFunction|ExRecordPlayback))))

(fn ExModifyOption
  (bind _returnvalue (Class|RealSenseContext|GetDevicebyId (Variables|Default|GetContext)))
  (bind _returnvalue_2 (Class|RealSenseDevice|GetSensor _returnvalue "STREAM_COLOR"))
  (bind _returnvalue_3 (Class|RealSenseSensor|GetOption _returnvalue_2 "CONTRAST"))
  (Class|RealSenseOption|SetValue _returnvalue_3 (.Default (Utilities|Struct|BreakRealSenseOptionRange (Variables|/Script/RealSense.RealSenseOption|GetRange _returnvalue_3)))))

(fn ExPresetLoadSave
  (bind _returnvalue (Utilities|String|MakeLiteralString "test_preset.json"))
  (bind _returnvalue_2 (Class|RealSenseContext|GetDevicebyId (Variables|Default|GetContext)))
  (Class|RealSenseDevice|SavePreset _returnvalue_2 _returnvalue)
  (Class|RealSenseDevice|LoadPreset _returnvalue_2 _returnvalue))

(fn RunRealSenseDemo
  (bind _inspector (Variables|Default|GetInspector))
  (Class|RealSenseInspector|Start _inspector)
  (Default|SetupDemoObjects _inspector))

(fn ExRecordPlayback
  (bind _inspector (Variables|Default|GetInspector))
  (Variables|/Script/RealSense.RealSenseInspector|SetPipelineMode _inspector "RecordFile")
  (Variables|/Script/RealSense.RealSenseInspector|SetCaptureFile _inspector "test_record.bin")
  (Class|RealSenseInspector|Start _inspector)
  (Utilities|Time|SetTimerbyFunctionName self "OnRecordCompleted" 1e+01))

(fn InitInspector
  (Utilities|IsValid (Variables|Default|GetInspector)
    (:Is%20Not%20Valid
      (bind _outactors (Actor|GetAllActorsOfClass "/Game/BP_RealSenseInspector.BP_RealSenseInspector_C"))
      (Variables|Default|SetInspector (Utilities|Array|Get(acopy) _outactors)))))

(fn OnRecordCompleted
  (bind _inspector (Variables|Default|GetInspector))
  (Class|RealSenseInspector|Stop _inspector)
  (Variables|/Script/RealSense.RealSenseInspector|SetPipelineMode _inspector "PlaybackFile")
  (Variables|/Script/RealSense.RealSenseInspector|SetCaptureFile _inspector "test_record.bin")
  (Class|RealSenseInspector|Start _inspector)
  (Utilities|Time|SetTimerbyFunctionName self "OnPlaybackCompleted" 1e+01))

(fn OnPlaybackCompleted
  (bind _inspector (Variables|Default|GetInspector))
  (Class|RealSenseInspector|Stop _inspector)
  (Variables|/Script/RealSense.RealSenseInspector|SetPipelineMode _inspector "CaptureOnly"))

(fn ExStreamConfiguration
  (bind _realsensestreammode (Utilities|Struct|MakeRealSenseStreamMode 848 480 15))
  (bind _inspector (Variables|Default|GetInspector))
  (Variables|/Script/RealSense.RealSenseInspector|SetDepthConfig _inspector _realsensestreammode)
  (Variables|/Script/RealSense.RealSenseInspector|SetInfraredConfig _inspector _realsensestreammode)
  (Variables|/Script/RealSense.RealSenseInspector|SetColorConfig _inspector (Utilities|Struct|MakeRealSenseStreamMode 1280 720 15))
  (Variables|/Script/RealSense.RealSenseInspector|SetbEnablePcl _inspector false))